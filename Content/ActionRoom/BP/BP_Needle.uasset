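; BP_Needle is an ActionRoom actor that lays out a grid of static meshes, presumably needles.
; The construction script calls the parent script, then runs nested loops over X and Y, adding a mesh component at each cell with 100-unit spacing.
; The event graph holds only disabled placeholder events, so this Blueprint adds no runtime logic of its own.
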(fn `UserConstructionScript`
  (`parent.UserConstructionScript`)
  (for _index (range 1 (+ (`self.X`) 1))
    (for _index_2 (range 1 (+ (`self.Y`) 1))
      (`AddComponent|NODE_AddStaticMeshComponent-0` :`RelativeTransform` (`KismetMathLibrary.MakeTransform` (`KismetMathLibrary.MakeVector` (`KismetMathLibrary.Conv_IntToDouble` (* (- _index 1) 100)) (`KismetMathLibrary.Conv_IntToDouble` (* (- _index_2 1) 100))))))))