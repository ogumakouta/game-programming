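; BP_FE_WeightSwitch is a one-shot pressure plate that opens its SecurityGate when a BP_FE_FallingCube rests in or enters its TriggerBox, marked as protected exam infrastructure.
; Tick looks up a falling cube with GetActorOfClass and polls the box for overlap, rather than using overlap events.
; The first hit latches Activated, moves PlateMesh to its relative origin and calls OpenGate, with no reset.
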(event `self.ReceiveTick`
  (params (DeltaSeconds :type "Float (single-precision)"))
  (`|ExecutionSequence`
    (:`then_0`
      (bind _returnvalue (`GameplayStatics.GetActorOfClass` "/Game/FinalExam/StudentWork/BP_FE_FallingCube.BP_FE_FallingCube_C"))
      (bind _asbp_fe_falling_cube (cast `/Game/FinalExam/StudentWork/BP_FE_FallingCube` _returnvalue))
      (if (`PrimitiveComponent.IsOverlappingActor` (`self.TriggerBox`) _asbp_fe_falling_cube)
        (if (not (`self.bActivated`))
          (set `self.bActivated` true)
          (`SceneComponent.K2_SetRelativeLocation` (`self.PlateMesh`) (0.0 0.0 0.0) false false)
          (`/Game/FinalExam/Infrastructure/BP_FE_SecurityGate.OpenGate` (`self.SecurityGate`)))))))

(fn `UserConstructionScript`)