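; BP_Goal is a goal trigger that stages the finish when the player character reaches it.
; When GoalCollision begins overlapping the player character, it spawns a RadialBurst effect and plays a click sound at the player's location.
; It then adds the WBP_Goal widget to the viewport, disables the player character's input and plays the sequence referenced by GoalSequencer.
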(event `self.GoalCollision.OnComponentBeginOverlap`
  (params (OverlappedComponent :type "PrimitiveComponent Object Reference") (OtherActor :type "Actor Object Reference") (OtherComp :type "PrimitiveComponent Object Reference") (OtherBodyIndex :type Integer) (bFromSweep :type Boolean) (SweepResult :type "HitResult Structure (by ref)"))
  (bind _returnvalue (`self.K2_GetActorLocation` OtherActor))
  (if (== OtherActor (`GameplayStatics.GetPlayerCharacter` 0))
    (`NiagaraFunctionLibrary.SpawnSystemAtLocation` "/Niagara/DefaultAssets/Templates/Systems/RadialBurst.RadialBurst" _returnvalue)
    (`GameplayStatics.PlaySoundAtLocation` "/Engine/VREditor/Sounds/VR_click3.VR_click3" _returnvalue (struct) 1.0 1.0 0.0 null null null null)
    (bind _returnvalue_2 (`|CreateWidget` "/Game/FirstProject/UI/WBP_Goal.WBP_Goal_C"))
    (`UserWidget.AddToViewport` _returnvalue_2 0)
    (`self.DisableInput` (`GameplayStatics.GetPlayerCharacter` 0) (`GameplayStatics.GetPlayerController` 0))
    (`MovieSceneSequencePlayer.Play` (`LevelSequenceActor.SequencePlayer` (`self.GoalSequencer`)))))

(fn `UserConstructionScript`)