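; BP_Switch_Base is a base pushbutton switch actor that sinks when the third-person player character hits its Button component.
; An IsPressed flag guards against retriggering while the ButtonUpDown timeline lowers the button along Z.
; When the timeline finishes, its direction selects OnPressedButton, an empty hook, or OnReleasedButton, which clears the flag.
; Nothing in this Blueprint plays the timeline in reverse.
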(event `self.Button.OnComponentHit`
  (params (HitComponent :type "PrimitiveComponent Object Reference") (OtherActor :type "Actor Object Reference") (OtherComp :type "PrimitiveComponent Object Reference") (NormalImpulse :type "Vector Structure") (Hit :type "HitResult Structure (by ref)"))
  ; 人間が当たったかどうかの判定
  (cast `/Game/ThirdPerson/Blueprints/BP_ThirdPersonCharacter` OtherActor)
  ; まだボタンを押してなければ押したことにする
  (if (not (`self.IsPressed`))
    (set `self.IsPressed` true)
    (bind (_direction _height) (`Timeline|ButtonUpDown` :!via `PlayFromStart`)
      (:`Update`
        (`SceneComponent.K2_SetRelativeLocation` (`self.Button`) (`KismetMathLibrary.MakeVector` 0.0 0.0 (`KismetMathLibrary.MapRangeClamped` _height 0.0 1.0 35.0 15.0)) false false))
      (:`Finished`
        (if (`|EnumEquality` _direction "Forward")
          (`self.On Pressed Button`)
          (else
            (`self.On Released Button`)))))))

(event `On Pressed Button`)

(event `On Released Button`
  (set `self.IsPressed` false))

(fn `UserConstructionScript`)